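; Enemy turret actor that fires projectiles on a repeating timer while a timeline moves it along the vertical axis.
; BeginPlay starts the looping shot timer, stores the starting position and plays the Cronograma timeline, whose Movement track offsets the actor's Z from that position.
; Each shot spawns an EnemyBullet at ShootPoint, aimed by rotating the forward vector by ProjectileDirection, then sets its speed and plays a firing sound.
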(event Custom|Shoot
  (bind _returnvalue (Game|SpawnActorfromClass "/Game/Blueprints/EnemyBullet.EnemyBullet_C" (Math|Transform|MakeTransform (Transformation|GetWorldLocation (Variables|Default|GetShootPoint)) (Math|Conversions|RotationFromXVector (Math|Vector|RotateVector (Transformation|GetActorForwardVector) (Variables|Default|GetProjectileDirection))) "1.000000,1.000000,1.000000") "Undefined" "MultiplyWithRoot" 0 0))
  (Variables|/Game/Blueprints/Bullet.Bullet_C|SetProjectileSpeed _returnvalue (Variables|Default|GetProjectileSpeed))
  (Audio|PlaySound2D "/Game/Sounds/DisparoAliado.DisparoAliado" 0.1 1.0 0.0 0 0))

(event EventBeginPlay
  (Utilities|Time|SetTimerbyEvent (delegate Custom|Shoot) (Variables|Default|GetShootingSpeed) true)
  (Variables|Default|SetStartingPosition (Transformation|GetActorLocation))
  (bind _movement (Timeline|Cronograma Play)
    (:Update
      (Transformation|SetActorLocation (+ (Math|Vector|MakeVector 0.0 0.0 _movement) (Variables|Default|GetStartingPosition)) false false))))

(event EventTick
  (params (DeltaSeconds :type Float%20%28single-precision%29)))

(fn ConstructionScript)