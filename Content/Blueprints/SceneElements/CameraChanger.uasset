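; CameraChanger is an overlap-triggered actor that switches the player's view and can act as a save point.
; After a short delay, a Player-tagged overlap blends the view to its assigned Camera, or to the player character if none is valid.
; When SaveGame is set, any overlapping BP_ThirdPersonCharacter, tagged or not, saves its position, then every Door actor saves its state.
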(event Collision|EventActorBeginOverlap
  (params (OtherActor :type Actor%20Object%20Reference))
  (bind _returnvalue (Game|GetPlayerController 0))
  (bind _camera (Variables|Default|GetCamera))
  (Utilities|FlowControl|Delay 0.2)
  (if (Actor|ActorHasTag OtherActor "Player")
    (if (Utilities|IsValid _camera)
      (Game|Player|SetViewTargetwithBlend _returnvalue _camera 1.5 "VTBlend_Linear" 0.0 false)
      (else
        (bind _asbp_third_person_character (Utilities|Casting|CastToBP_ThirdPersonCharacter (Game|GetPlayerCharacter 0)))
        (Game|Player|SetViewTargetwithBlend _returnvalue _asbp_third_person_character 1.5 "VTBlend_Linear" 0.0 false))))
  (if (Variables|Default|GetSaveGame)
    (bind _asbp_third_person_character_2 (Utilities|Casting|CastToBP_ThirdPersonCharacter OtherActor))
    (Default|SavePosition _asbp_third_person_character_2)
    (bind _outactors (Actor|GetAllActorsOfClass "/Game/Blueprints/SceneElements/Door.Door_C"))
    (for _array_element _outactors
      (Default|SaveDoors _array_element))))

(fn ConstructionScript)