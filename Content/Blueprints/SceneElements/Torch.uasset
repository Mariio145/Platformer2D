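; Torch actor that a fireball can light once as part of a linked Door's opening logic.
; It registers with the Door on BeginPlay and, after a short delay, switches to its lit components if the Door is already open.
; An overlap by an actor tagged Fireball swaps the mesh material to fire, notifies the Door, destroys the Bullet and shows the lit components.
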(event Collision|EventActorBeginOverlap
  (params (OtherActor :type Actor%20Object%20Reference))
  (if (not (Variables|Default|GetAlreadyUsed))
    (if (Actor|ActorHasTag OtherActor "Fireball")
      (Variables|Default|SetAlreadyUsed true)
      (Rendering|Material|SetMaterial (Variables|Default|GetTorchMesh) 1 "/Game/Fab/MedievalModels/Fire.Fire")
      (Default|TorchLitUp (Variables|Default|GetDoor))
      (bind _asbullet (Utilities|Casting|CastToBullet OtherActor))
      (Default|Destroy _asbullet)
      (Development|SetHiddeninGame (Variables|Default|GetPostLit) false false)
      (Development|SetHiddeninGame (Variables|Default|GetPretLit) true false))))

(event EventBeginPlay
  (bind _door (Variables|Default|GetDoor))
  (Development|SetHiddeninGame (Variables|Default|GetPostLit) true false)
  (Default|AddTorch _door)
  (Utilities|FlowControl|Delay 0.2)
  (if (Variables|/Game/Blueprints/SceneElements/Door.Door_C|GetOpened _door)
    (Variables|Default|SetAlreadyUsed true)
    (Development|SetHiddeninGame (Variables|Default|GetPostLit) false false)
    (Development|SetHiddeninGame (Variables|Default|GetPretLit) true false)))

(fn ConstructionScript)