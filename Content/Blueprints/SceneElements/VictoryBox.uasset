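; VictoryBox is the level's win trigger, reacting when the third-person player character overlaps it.
; On overlap it rotates the character by a fixed offset and plays a victory montage on its mesh.
; As the montage starts, it disables input, shows the win text, hides the staff and plays a victory sound.
; When the montage completes, it opens the main menu level.
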(event Collision|EventActorBeginOverlap
  (params (OtherActor :type Actor%20Object%20Reference))
  (bind _asbp_third_person_character (Utilities|Casting|CastToBP_ThirdPersonCharacter OtherActor))
  (Transformation|SetActorRotation _asbp_third_person_character (Math|Rotator|CombineRotators (Transformation|GetActorRotation _asbp_third_person_character) "0.000000,120.000000,0.000000") true)
  (Animation|Montage|PlayMontage (Variables|/Script/Engine.Character|GetMesh _asbp_third_person_character) "/Game/AnimationRetargeted/Montages/VictoryMontage.VictoryMontage"
    (:then
      (Input|DisableInput _asbp_third_person_character 0)
      (Default|ShowText _asbp_third_person_character "You Won!" 3.0)
      (Development|SetHiddeninGame (Variables|/Game/Blueprints/BP_ThirdPersonCharacter.BP_ThirdPersonCharacter_C|GetStaff _asbp_third_person_character) true false)
      (Audio|PlaySound2D "/Game/Sounds/Victoria.Victoria" 0.6 1.0 0.0 0 0))
    (:OnCompleted
      (Game|OpenLevel(byName) "MainMenu"))))

(fn ConstructionScript)