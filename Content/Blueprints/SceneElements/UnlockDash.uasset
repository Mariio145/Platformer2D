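; Pickup actor that grants the player the dash ability in BP_ThirdPersonCharacter.
; Shortly after BeginPlay it destroys itself if the player already has dash, otherwise it animates vertically from its start position with a timeline.
; Overlap by an actor tagged Player sets HasDash, destroys the pickup and shows an on-screen message that dashing is unlocked.
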(event EventBeginPlay
  (bind _asbp_third_person_character (Utilities|Casting|CastToBP_ThirdPersonCharacter (Game|GetPlayerCharacter 0)))
  (Utilities|FlowControl|Delay 0.2)
  (if (Variables|/Game/Blueprints/BP_ThirdPersonCharacter.BP_ThirdPersonCharacter_C|GetHasDash _asbp_third_person_character)
    (Actor|DestroyActor)
    (else
      (Variables|Default|SetStartingPosition (Transformation|GetActorLocation))
      (bind _movement (Timeline|moving Play)
        (:Update
          (Transformation|SetActorLocation (+ (Math|Vector|MakeVector 0.0 0.0 _movement) (Variables|Default|GetStartingPosition)) false false))))))

(event Collision|EventActorBeginOverlap
  (params (OtherActor :type Actor%20Object%20Reference))
  (if (Actor|ActorHasTag OtherActor "Player")
    (bind _asbp_third_person_character (Utilities|Casting|CastToBP_ThirdPersonCharacter OtherActor))
    (Variables|/Game/Blueprints/BP_ThirdPersonCharacter.BP_ThirdPersonCharacter_C|SetHasDash _asbp_third_person_character true)
    (Actor|DestroyActor)
    (Default|ShowText _asbp_third_person_character "Now you can dash!" 3.0)))

(fn ConstructionScript)