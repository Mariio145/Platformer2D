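; Barred door actor that opens by raising its bars on a timeline with a sound, once all registered torches are lit.
; Torches register through AddTorch and report through TorchLitUp, which compares the lit count to the total.
; On BeginPlay it reopens if the save slot flags its DoorType as open, and SaveDoors writes that state back.
; A door marked FirstDoor shows a crouch hint after opening.
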(event Custom|AddTorch
  (Variables|Default|SetTotalNumTorches (+ 1 (Variables|Default|GetTotalNumTorches))))

(event Custom|TorchLitUp
  (Variables|Default|SetTorchesActivated (+ 1 (Variables|Default|GetTorchesActivated)))
  (if (>= (Variables|Default|GetTorchesActivated) (Variables|Default|GetTotalNumTorches))
    (Audio|PlaySound2D "/Game/Sounds/OpenDoor.OpenDoor" 0.5 1.0 4.0 0 0)
    (Variables|Default|SetOpened true)
    (bind _opensequence (Timeline|Open%20Door Play)
      (:Update
        (Transformation|SetRelativeLocation (Variables|Default|GetBars) (Math|Vector|MakeVector 0.0 0.0 (Math|Float|Lerp 0.0 1.5e+02 _opensequence)) false false))
      (:Finished
        (if (Variables|Default|GetFirstDoor)
          (bind _asbp_third_person_character (Utilities|Casting|CastToBP_ThirdPersonCharacter (Game|GetPlayerCharacter 0)))
          (Default|ShowText _asbp_third_person_character "Press CTRL to crouch" 3.5))))))

(event Custom|OpenDoor
  (Audio|PlaySound2D "/Game/Sounds/OpenDoor.OpenDoor" 0.5 1.0 4.0 0 0)
  (Variables|Default|SetOpened true)
  (bind _opensequence (Timeline|Open%20Door Play)
    (:Update
      (Transformation|SetRelativeLocation (Variables|Default|GetBars) (Math|Vector|MakeVector 0.0 0.0 (Math|Float|Lerp 0.0 1.5e+02 _opensequence)) false false))
    (:Finished
      (if (Variables|Default|GetFirstDoor)
        (bind _asbp_third_person_character (Utilities|Casting|CastToBP_ThirdPersonCharacter (Game|GetPlayerCharacter 0)))
        (Default|ShowText _asbp_third_person_character "Press CTRL to crouch" 3.5)))))

(event EventBeginPlay
  (bind _asbp_third_person_game_instance (Utilities|Casting|CastToBP_ThirdPersonGameInstance (Game|GetGameInstance)))
  (bind _returnvalue (SaveGame|LoadGamefromSlot (Variables|/Game/Blueprints/BP_ThirdPersonGameInstance.BP_ThirdPersonGameInstance_C|GetSlotName _asbp_third_person_game_instance) (Variables|/Game/Blueprints/BP_ThirdPersonGameInstance.BP_ThirdPersonGameInstance_C|GetSlot _asbp_third_person_game_instance)))
  (bind _asbp_third_person_save_game (Utilities|Casting|CastToBP_ThirdPersonSaveGame _returnvalue))
  (switch Utilities|FlowControl|Switch|SwitchonDoorEnum (Variables|Default|GetDoorType)
    (:NewEnumerator0
      (if (Variables|/Game/Blueprints/BP_ThirdPersonSaveGame.BP_ThirdPersonSaveGame_C|Get2DoorOpen _asbp_third_person_save_game)
        (CallFunction|OpenDoor :!label _label)))
    (:NewEnumerator1
      (if (Variables|/Game/Blueprints/BP_ThirdPersonSaveGame.BP_ThirdPersonSaveGame_C|Get3DoorOpen _asbp_third_person_save_game)
        (goto _label)))
    (:NewEnumerator2
      (if (Variables|/Game/Blueprints/BP_ThirdPersonSaveGame.BP_ThirdPersonSaveGame_C|Get1DoorOpen _asbp_third_person_save_game)
        (goto _label)))))

(event Collision|EventActorBeginOverlap
  (params (OtherActor :type Actor%20Object%20Reference)))

(event EventTick
  (params (DeltaSeconds :type Float%20%28single-precision%29)))

(fn ConstructionScript)

(fn SaveDoors
  (bind _opened (Variables|Default|GetOpened))
  (bind _asbp_third_person_game_instance (Utilities|Casting|CastToBP_ThirdPersonGameInstance (Game|GetGameInstance)))
  (bind _returnvalue (SaveGame|DoesSaveGameExist (Variables|/Game/Blueprints/BP_ThirdPersonGameInstance.BP_ThirdPersonGameInstance_C|GetSlotName _asbp_third_person_game_instance) (Variables|/Game/Blueprints/BP_ThirdPersonGameInstance.BP_ThirdPersonGameInstance_C|GetSlot _asbp_third_person_game_instance)))
  (if _returnvalue
    (bind _returnvalue_2 (SaveGame|LoadGamefromSlot (Variables|/Game/Blueprints/BP_ThirdPersonGameInstance.BP_ThirdPersonGameInstance_C|GetSlotName _asbp_third_person_game_instance) (Variables|/Game/Blueprints/BP_ThirdPersonGameInstance.BP_ThirdPersonGameInstance_C|GetSlot _asbp_third_person_game_instance)))
    (bind _asbp_third_person_save_game (Utilities|Casting|CastToBP_ThirdPersonSaveGame _returnvalue_2))
    (switch Utilities|FlowControl|Switch|SwitchonDoorEnum (Variables|Default|GetDoorType)
      (:NewEnumerator0
        (Variables|/Game/Blueprints/BP_ThirdPersonSaveGame.BP_ThirdPersonSaveGame_C|Set2DoorOpen _asbp_third_person_save_game _opened))
      (:NewEnumerator1
        (Variables|/Game/Blueprints/BP_ThirdPersonSaveGame.BP_ThirdPersonSaveGame_C|Set3DoorOpen _asbp_third_person_save_game _opened))
      (:NewEnumerator2
        (Variables|/Game/Blueprints/BP_ThirdPersonSaveGame.BP_ThirdPersonSaveGame_C|Set1DoorOpen _asbp_third_person_save_game _opened)))
    (SaveGame|SaveGametoSlot _asbp_third_person_save_game (Variables|/Game/Blueprints/BP_ThirdPersonGameInstance.BP_ThirdPersonGameInstance_C|GetSlotName _asbp_third_person_game_instance) (Variables|/Game/Blueprints/BP_ThirdPersonGameInstance.BP_ThirdPersonGameInstance_C|GetSlot _asbp_third_person_game_instance))))