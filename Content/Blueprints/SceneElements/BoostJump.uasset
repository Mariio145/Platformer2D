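; BoostJump is a pickup actor that raises the player character's jump velocity.
; On begin play, the Moving timeline offsets it vertically from its starting position.
; When a Player-tagged actor overlaps it, it multiplies that BP_ThirdPersonCharacter's JumpZVelocity, destroys itself and shows a short on-screen message.
; The boost has no reset here, so repeated pickups compound.
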(event EventBeginPlay
  (Variables|Default|SetStartingPosition (Transformation|GetActorLocation))
  (bind _movement (Timeline|moving Play)
    (:Update
      (Transformation|SetActorLocation (+ (Math|Vector|MakeVector 0.0 0.0 _movement) (Variables|Default|GetStartingPosition)) false false))))

(event Collision|EventActorBeginOverlap
  (params (OtherActor :type Actor%20Object%20Reference))
  (if (Actor|ActorHasTag OtherActor "Player")
    (bind _asbp_third_person_character (Utilities|Casting|CastToBP_ThirdPersonCharacter OtherActor))
    (Variables|/Script/Engine.CharacterMovementComponent|SetJumpZVelocity (Variables|/Script/Engine.Character|GetCharacterMovement _asbp_third_person_character) (* (Variables|/Script/Engine.CharacterMovementComponent|GetJumpZVelocity (Variables|/Script/Engine.Character|GetCharacterMovement _asbp_third_person_character)) 1.2))
    (Actor|DestroyActor)
    (Default|ShowText _asbp_third_person_character "Now you jump even more!" 3.0)))

(fn ConstructionScript)