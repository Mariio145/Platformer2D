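; SwitchPlatform is a scene element platform that alternates between solid and passable on a fixed cycle.
; A looping timer started at BeginPlay fires Switch, which flips the UpNow flag and sets the root component's active state to match.
; When up, the FloorModular mesh shows the grey floor material with query and physics collision; when down, it shows the disc material with collision disabled.
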(event Custom|Switch
  (bind _floor_modular (Variables|Default|GetFloor_Modular))
  (bind _output_get (Variables|Default|SetUpNow (not (Variables|Default|GetUpNow))))
  (Components|Activation|SetActive (Variables|Default|GetDefaultSceneRoot) _output_get false)
  (if (Variables|Default|GetUpNow)
    (Rendering|Material|SetMaterial (Variables|Default|GetFloor_Modular) 0 "/Game/Fab/MedievalModels/Grey_Floor.Grey_Floor")
    (Collision|SetCollisionEnabled _floor_modular "QueryAndPhysics")
    (else
      (Rendering|Material|SetMaterial (Variables|Default|GetFloor_Modular) 0 "/Engine/VREditor/UI/DiscMaterial.DiscMaterial")
      (Collision|SetCollisionEnabled _floor_modular "NoCollision"))))

(event EventBeginPlay
  (Utilities|Time|SetTimerbyEvent (delegate Custom|Switch) 3.0 true))

(fn ConstructionScript)